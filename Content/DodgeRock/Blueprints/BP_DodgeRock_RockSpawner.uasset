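; Rock spawner actor for DodgeRock that drops new rock actors at random positions within its Box component's footprint.
; On BeginPlay it reads the difficulty from the game instance and picks a matching stone damage value.
; SpawnStone, an event with no caller in this file, randomizes X and Y inside the box, keeps the spawner's height, and passes that damage to each rock as BaseDamage.
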(event `self.ReceiveBeginPlay`
  (bind _asbp_dodge_rock_game_instance (cast `/Game/DodgeRock/Core/GameInstance/BP_DodgeRock_GameInstance` (`GameplayStatics.GetGameInstance`)))
  (set `self.StoneDamageModifier` (select `/Game/DodgeRock/Enums/E_GameDifficulty` (`/Game/DodgeRock/Core/GameInstance/BP_DodgeRock_GameInstance.GetDifficulty` _asbp_dodge_rock_game_instance) :`NewEnumerator0` 25.0 :`NewEnumerator1` 50.0 :`NewEnumerator2` 100.0)))

(event `SpawnStone`
  (bind _box (`self.Box`))
  (`|SpawnActorFromClass` "/Game/DodgeRock/Blueprints/BP_DodgeRock_Rock.BP_DodgeRock_Rock_C" (`KismetMathLibrary.MakeTransform` (`KismetMathLibrary.MakeVector` (.x (`KismetMathLibrary.RandomPointInBoundingBox` (`SceneComponent.K2_GetComponentLocation` _box) (`BoxComponent.GetScaledBoxExtent` _box))) (.y (`KismetMathLibrary.RandomPointInBoundingBox` (`SceneComponent.K2_GetComponentLocation` _box) (`BoxComponent.GetScaledBoxExtent` _box))) (.z (`self.K2_GetActorLocation`)))) "AdjustIfPossibleButAlwaysSpawn" "MultiplyWithRoot" null (`self.StoneDamageModifier`) null))

(fn `UserConstructionScript`)