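; BP_HealthComponent is an actor component that tracks health for its owning actor in DodgeRock.
; On BeginPlay it binds to the owner's OnTakeAnyDamage event and sets health to the default value.
; Each hit subtracts damage, clamped between zero and current health, and fires the OnOwnerDied dispatcher when health reaches zero.
; Simple getters and setters expose current and default health.
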(event `self.ReceiveBeginPlay`
  (add `Actor.OnTakeAnyDamage` (`self.GetOwner`) (`|CreateDelegate` :!event `OnTakeAnyDamage_Event`))
  (`self.SetHealth` (`self.DefaultHealth`)))

(event `OnTakeAnyDamage_Event`
  (params (DamagedActor :type "Actor Object Reference") (Damage :type "Float (single-precision)") (DamageType :type "DamageType Object Reference") (InstigatedBy :type "Controller Object Reference") (DamageCauser :type "Actor Object Reference"))
  (bind _newparam (`self.GetHealth`))
  (`self.SetHealth` (`KismetMathLibrary.FClamp` (- _newparam Damage) 0.0 _newparam))
  (if (<= (`self.GetHealth`) 0.0)
    (`self.OnOwnerDied`)))

(fn `GetDefaultHealth`
  (returns (deafaultHealth :type "Float (double-precision)"))
  (return (`self.DefaultHealth`)))

(fn `GetHealth`
  (returns (NewParam :type "Float (double-precision)"))
  (return (`self.Health`)))

(fn `SetDefaultHealth`
  (params (DefaultHealth :type "Float (double-precision)"))
  (set `self.DefaultHealth` DefaultHealth))

(fn `SetHealth`
  (params (`New Health` :type "Float (double-precision)"))
  (set `self.Health` `New Health`))