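; Player controller for the DodgeRock character, handling movement, look, jump and pause input.
; On BeginPlay it sets game-only input, adds the Enhanced Input mapping context and caches the controlled character and its movement component.
; Movement input is applied along control-rotation directions straight to the movement component.
; The pause action toggles game pause, lazily creating a reusable pause menu widget and switching input mode and cursor visibility.
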(event `self.ReceiveBeginPlay`
  (`WidgetBlueprintLibrary.SetInputMode_GameOnly` self)
  (set `self.bShowMouseCursor` false)
  (`EnhancedInputSubsystemInterface.AddMappingContext` (subsystem `EnhancedInputLocalPlayerSubsystem`) "/Game/DodgeRock/Core/Input/IMC_DodgeRock_PlayerInput.IMC_DodgeRock_PlayerInput" 0 (struct))
  (bind _asbp_dodge_rock_character (cast `/Game/DodgeRock/Characters/BP_DodgeRock_Character` (`self.K2_GetPawn`)))
  (bind _output_get (set `self.Dodge Rock Character` _asbp_dodge_rock_character))
  (set `self.Character Movement Comp` (`Character.CharacterMovement` _output_get)))

(event `EnhancedInput|/Game/DodgeRock/Core/Input/Actions/IA_DodgeRockMoving`
  (params (ActionValue :type "Vector2D Structure") (ElapsedSeconds :type "Float (double-precision)") (TriggeredSeconds :type "Float (double-precision)") (InputAction :type "InputAction Object Reference" :default "/Game/DodgeRock/Core/Input/Actions/IA_DodgeRockMoving.IA_DodgeRockMoving"))
  (bind (_returnvalue_roll _returnvalue_pitch _returnvalue_yaw) (`KismetMathLibrary.BreakRotator` (`self.GetControlRotation`)))
  (bind (_returnvalue_roll_2 _returnvalue_pitch_2 _returnvalue_yaw_2) (`KismetMathLibrary.BreakRotator` (`self.GetControlRotation`)))
  (:`Triggered`
    (bind _character_movement_comp (`self.Character Movement Comp`)
      (:`then`
        (`|ExecutionSequence`
          (:`then_0`
            (`PawnMovementComponent.AddInputVector` _character_movement_comp (* (`KismetMathLibrary.GetForwardVector` (`KismetMathLibrary.MakeRotator` 0.0 0.0 _returnvalue_yaw_2)) ActionValue_Y) false))
          (:`then_1`
            (`PawnMovementComponent.AddInputVector` _character_movement_comp (* (`KismetMathLibrary.GetRightVector` (`KismetMathLibrary.MakeRotator` _returnvalue_roll 0.0 _returnvalue_yaw)) ActionValue_X) false))))
      (:`else`))))

(event `EnhancedInput|/Game/DodgeRock/Core/Input/Actions/IA_DodgeRockLook`
  (params (ActionValue :type "Vector2D Structure") (ElapsedSeconds :type "Float (double-precision)") (TriggeredSeconds :type "Float (double-precision)") (InputAction :type "InputAction Object Reference" :default "/Game/DodgeRock/Core/Input/Actions/IA_DodgeRockLook.IA_DodgeRockLook"))
  (:`Triggered`
    (`self.Character Movement Comp`
      (:`then`
        (`self.AddYawInput` ActionValue_X)
        (`self.AddPitchInput` ActionValue_Y))
      (:`else`))))

(event `EnhancedInput|/Game/DodgeRock/Core/Input/Actions/IA_DodgeRockJump`
  (params (ActionValue :type Boolean) (ElapsedSeconds :type "Float (double-precision)") (TriggeredSeconds :type "Float (double-precision)") (InputAction :type "InputAction Object Reference" :default "/Game/DodgeRock/Core/Input/Actions/IA_DodgeRockJump.IA_DodgeRockJump"))
  (:`Triggered`
    (bind _dodge_rock_character (`self.Dodge Rock Character`)
      (:`then`
        (`Character.Jump` _dodge_rock_character))
      (:`else`)))
  (:`Completed`
    (`Character.StopJumping` _dodge_rock_character)))

(event `EnhancedInput|/Game/DodgeRock/Core/Input/Actions/IA_DodgeRockPause`
  (params (ActionValue :type Boolean) (ElapsedSeconds :type "Float (double-precision)") (TriggeredSeconds :type "Float (double-precision)") (InputAction :type "InputAction Object Reference" :default "/Game/DodgeRock/Core/Input/Actions/IA_DodgeRockPause.IA_DodgeRockPause"))
  (:`Triggered`
    (if (`GameplayStatics.IsGamePaused`)
      (`GameplayStatics.SetGamePaused` false)
      (`WidgetBlueprintLibrary.SetInputMode_GameOnly` self)
      (set `self.bShowMouseCursor` false)
      (bind _pausemenuwidget (`self.PauseMenuWidget`)
        (:`then`
          (`Widget.RemoveFromParent` _pausemenuwidget))
        (:`else`))
      (else
        (`GameplayStatics.SetGamePaused` true)
        (`self.PauseMenuWidget`
          (:`then`
            _)
          (:`else`
            (bind _returnvalue (`|CreateWidget` "/Game/DodgeRock/UI/WBP_DodgeRock_PauseMenu.WBP_DodgeRock_PauseMenu_C" self))
            (bind _output_get (set `self.PauseMenuWidget` _returnvalue))))
        (`UserWidget.AddToViewport` _output_get 0)
        (`WidgetBlueprintLibrary.SetInputMode_GameAndUIEx` self _output_get)
        (set `self.bShowMouseCursor` true)))))

(fn `UserConstructionScript`)