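; Game instance for DodgeRock that holds the selected game difficulty and the highest score.
; Simple getter and setter functions expose both values.
; The high score setter overwrites the stored value only when the new score is greater.
; The file contains no save-to-disk logic.
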(fn `GetDifficulty`
  (returns (GameDifficulty :type "/Game/DodgeRock/Enums/E_GameDifficulty Enum"))
  (return (`self.GameDifficulty`)))

(fn `GetHighestScore`
  (returns (HighestScore :type Integer))
  (return (`self.HighestScore`)))

(fn `SetDifficulty`
  (params (GameDifficulty :type "/Game/DodgeRock/Enums/E_GameDifficulty Enum" :default "NewEnumerator0"))
  (set `self.GameDifficulty` GameDifficulty))

(fn `SetHighestScore`
  (params (NewScore :type Integer))
  (if (< (`self.HighestScore`) NewScore)
    (set `self.HighestScore` NewScore)))