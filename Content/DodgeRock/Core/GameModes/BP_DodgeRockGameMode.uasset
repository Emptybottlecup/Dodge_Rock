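; Game mode for DodgeRock that runs the match flow and drives periodic rock spawning.
; On BeginPlay it starts the game state and binds to the player's health component death event to end the game.
; Its Process event takes the current time and, on every fifth count, triggers the level's rock spawner and increments the game state's rock count.
; Restart and End forward to the game state.
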(event `self.ReceiveBeginPlay`
  (`|ExecutionSequence`
    (:`then_0`
      (bind _asbp_dodge_rock_game_state (cast `/Game/DodgeRock/Core/GameState/BP_DodgeRock_GameState` (`GameplayStatics.GetGameState`)))
      (bind _output_get (set `self.Game State` _asbp_dodge_rock_game_state))
      (`/Game/DodgeRock/Core/GameState/BP_DodgeRock_GameState.Start` _output_get))
    (:`then_1`
      (bind _asbp_dodge_rock_character (cast `/Game/DodgeRock/Characters/BP_DodgeRock_Character` (`GameplayStatics.GetPlayerPawn` 0)))
      (add `/Game/DodgeRock/Blueprints/ActorComponents/BP_HealthComponent.OnOwnerDied` (`/Game/DodgeRock/Characters/BP_DodgeRock_Character.BP_HealthComponent` _asbp_dodge_rock_character) (`|CreateDelegate` :!event `OnPlayerDied`)))))

(event `Process`
  (params (`Current Time` :type Integer))
  (if (== (mod `Current Time` 5) 0)
    (`self.SpawnRock`)
    (bind _game_state (`self.Game State`)
      (:`then`
        (bind _result (`/Engine/EditorBlueprintResources/StandardMacros.IncrementInt` (`/Game/DodgeRock/Core/GameState/BP_DodgeRock_GameState.GetRockCount` _game_state))
          (:`  `
            (`/Game/DodgeRock/Core/GameState/BP_DodgeRock_GameState.SetRockCount` _game_state _result))))
      (:`else`))))

(event `SpawnRock`
  (bind _returnvalue (`GameplayStatics.GetActorOfClass` "/Game/DodgeRock/Blueprints/BP_DodgeRock_RockSpawner.BP_DodgeRock_RockSpawner_C"))
  (`/Game/DodgeRock/Blueprints/BP_DodgeRock_RockSpawner.SpawnStone` _returnvalue))

(event `Restart`
  (bind _game_state (`self.Game State`)
    (:`then`
      (`/Game/DodgeRock/Core/GameState/BP_DodgeRock_GameState.Restart` _game_state))
    (:`else`)))

(event `End`
  (bind _game_state (`self.Game State`)
    (:`then`
      (`/Game/DodgeRock/Core/GameState/BP_DodgeRock_GameState.End` _game_state))
    (:`else`)))

(event `OnPlayerDied`
  (`self.End`))

(fn `UserConstructionScript`)