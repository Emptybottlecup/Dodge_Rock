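; Game state for the DodgeRock minigame that runs the match clock and drives scoring and round flow.
; Start launches a looping one-second timer that counts time played, adds the current rock count to the player's score and passes elapsed time to the game mode's Process.
; End stops the timer, submits the score to the game instance as highest, then after a delay asks the game mode to restart; Restart reloads the current level.
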(event `self.ReceiveBeginPlay`
  (`|ExecutionSequence`
    (:`then_0`
      (bind _asbp_dodge_rock_game_mode (cast `/Game/DodgeRock/Core/GameModes/BP_DodgeRockGameMode` (`GameplayStatics.GetGameMode`)))
      (set `self.DodgeRock GameMode` _asbp_dodge_rock_game_mode))
    (:`then_1`
      (bind _asbp_dodge_rock_player_state (cast `/Game/DodgeRock/Core/PlayerState/BP_DodgeRock_PlayerState` (`GameplayStatics.GetPlayerState` 0)))
      (set `self.DodgeRock PlayerState` _asbp_dodge_rock_player_state))))

(event `Start`
  (bind _returnvalue (`KismetSystemLibrary.K2_SetTimerDelegate` (`|CreateDelegate` :!event `CoreGameTimeEvent`) 1.0 true))
  (set `self.DodgeRock CoreGameTimer` _returnvalue)
  (set `self.IsGameEnd` false))

(event `End`
  (`KismetSystemLibrary.K2_ClearAndInvalidateTimerHandle` (`self.DodgeRock CoreGameTimer`))
  (set `self.IsGameEnd` true)
  (`|ExecutionSequence`
    (:`then_0`
      (bind _asbp_dodge_rock_game_instance (cast `/Game/DodgeRock/Core/GameInstance/BP_DodgeRock_GameInstance` (`GameplayStatics.GetGameInstance`)))
      (bind _dodgerock_playerstate (`self.DodgeRock PlayerState`)
        (:`then`
          (`/Game/DodgeRock/Core/GameInstance/BP_DodgeRock_GameInstance.SetHighestScore` _asbp_dodge_rock_game_instance (`/Game/DodgeRock/Core/PlayerState/BP_DodgeRock_PlayerState.GetPlayerScore` _dodgerock_playerstate)))
        (:`else`)))
    (:`then_1`
      (`KismetSystemLibrary.Delay` 3.0)
      (bind _dodgerock_gamemode (`self.DodgeRock GameMode`)
        (:`then`
          (`/Game/DodgeRock/Core/GameModes/BP_DodgeRockGameMode.Restart` _dodgerock_gamemode))
        (:`else`)))))

(event `Restart`
  (bind _returnvalue (`GameplayStatics.GetCurrentLevelName` true))
  (`GameplayStatics.OpenLevel` (`KismetStringLibrary.Conv_StringToName` _returnvalue)))

(event `CoreGameTimeEvent`
  (`/Engine/EditorBlueprintResources/StandardMacros.IncrementInt` (`self.TimePlayed`)
    (:`  `
      (`|ExecutionSequence`
        (:`then_0`
          (bind _dodgerock_playerstate (`self.DodgeRock PlayerState`)
            (:`then`
              (`/Game/DodgeRock/Core/PlayerState/BP_DodgeRock_PlayerState.SetPlayerScore` _dodgerock_playerstate (+ (`/Game/DodgeRock/Core/PlayerState/BP_DodgeRock_PlayerState.GetPlayerScore` _dodgerock_playerstate) (`self.RockCount`))))
            (:`else`)))
        (:`then_1`
          (bind _dodgerock_gamemode (`self.DodgeRock GameMode`)
            (:`then`
              (`/Game/DodgeRock/Core/GameModes/BP_DodgeRockGameMode.Process` _dodgerock_gamemode (`self.TimePlayed`)))
            (:`else`)))))))

(fn `GetRockCount`
  (returns (`Count Of Rocks` :type Integer))
  (return (`self.RockCount`)))

(fn `SetRockCount`
  (params (CountOfRocks :type Integer))
  (set `self.RockCount` CountOfRocks))

(fn `UserConstructionScript`)